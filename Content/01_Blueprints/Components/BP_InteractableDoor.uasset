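; Interactable door component that handles player interaction, with optional key locking.
; On interaction, a closed door that uses a key checks the player's KeyNames for its KeyName; keyless doors skip the check.
; Success sets the Open flag and plays a random open sound.
; A missing key or an already open door plays a random locked sound at the owner's location.
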(event EventOnInteractionBP
  (params (Player :type Player%20Character%20Object%20Reference))
  (bind _doorlockedsfxs (Variables|Default|GetDoorLockedSFXs))
  ;[1 1 1] Only open door if it hasn't been open yet
  (if (Variables|Default|GetbOpen)
    ;[1 1 1] If the player can't open the door, play random door locked sound at owner actor location
    (CallFunction|PlaySoundatOwnerLocation (Utilities|Array|Get(acopy) _doorlockedsfxs (Math|Random|RandomInteger (Utilities|Array|Length _doorlockedsfxs))) :!label _label)
    (else
      ;[1 1 1] Check if this door needs key
      (if (Variables|Default|GetbUsesKey)
        ;[1 1 1] Check if the player has the key to open this door
        (if (Utilities|Array|ContainsItem (Variables|/Script/MEDJD_Projeto1.PlayerCharacter|GetKeyNames Player) (Variables|Default|GetKeyName))
          _
          (else
            (goto _label))))
      (Variables|Default|SetbOpen true)
      ;[1 1 1] Play random door open sound at owner actor location
      (CallFunction|PlayRandomSFX))))