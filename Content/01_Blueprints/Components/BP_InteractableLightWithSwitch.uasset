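; Interactable light component that adds a visual switch flip to its parent's interaction behavior.
; On interaction it runs the parent logic, then rotates the referenced Switch 180 degrees in relative pitch.
; The Switch reference is supplied from outside through SetSwitchReference.
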(event EventBeginPlay
  (|CallParentFunction) ; This node is disabled and will not be called.\nDrag off pins to build functionality.
)

(event EventTick
  (params (DeltaSeconds :type Float%20%28single-precision%29))
  (|CallParentFunction DeltaSeconds) ; This node is disabled and will not be called.\nDrag off pins to build functionality.
)

(event EventOnInteractionBP
  (params (Player :type Player%20Character%20Object%20Reference))
  (bind _switch (Variables|Default|GetSwitch))
  (bind _relativerotation (Variables|/Script/Engine.SceneComponent|GetRelativeRotation _switch))
  (|CallParentFunction 0)
  (Transformation|SetRelativeRotation (Variables|Default|GetSwitch) (Math|Rotator|MakeRotator (.roll _relativerotation) (+ (.pitch _relativerotation) 1.8e+02) (.yaw _relativerotation)) false false))

(fn SetSwitchReference
  (params (SwitchRef :type Static%20Mesh%20Component%20Object%20Reference))
  (Variables|Default|SetSwitch SwitchRef))