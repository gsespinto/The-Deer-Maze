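; An interactable component that plays a random sound effect when its owner is interacted with.
; The interaction event picks a random entry from the SFXs array and plays it at the owning actor's location through a small helper function.
; BeginPlay and Tick are unused, so all behavior is driven by the interaction event.
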(event EventBeginPlay)

(event EventTick
  (params (DeltaSeconds :type Float%20%28single-precision%29)))

(event EventOnInteractionBP
  (params (Player :type Player%20Character%20Object%20Reference))
  (CallFunction|PlayRandomSFX))

(fn PlaySoundatOwnerLocation
  (params (Sound :type Sound%20Base%20Object%20Reference))
  (Audio|PlaySoundatLocation Sound (Transformation|GetActorLocation (Components|GetOwner)) "0, 0, 0" 1.0 1.0 0.0 0 0 0))

(fn PlayRandomSFX
  (bind _sfxs (Variables|Default|GetSFXs))
  (CallFunction|PlaySoundatOwnerLocation (Utilities|Array|Get(acopy) _sfxs (Math|Random|RandomInteger (Utilities|Array|Length _sfxs)))))