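; Interactable component for lore books that opens a reading widget and pauses the game.
; On interaction it waits briefly, plays a random book sound at the owner's location, then spawns the configured widget.
; The sound is flagged as a UI sound, so it keeps playing through the pause.
; ExitBook removes the widget and unpauses, acting only while a book is open.
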(event EventBeginPlay)

(event EventTick
  (params (DeltaSeconds :type Float%20%28single-precision%29)))

(event EventOnInteractionBP
  (params (Player :type Player%20Character%20Object%20Reference))
  (Utilities|FlowControl|Delay 0.5)
  (CallFunction|PlayBookSFX)
  (bind _returnvalue (UserInterface|CreateWidget (Variables|Default|GetWidgetToSpawn)))
  (bind _output_get (Variables|Default|SetWidgetRef _returnvalue))
  (UserInterface|Viewport|AddtoViewport _output_get 0)
  (Game|SetGamePaused true))

(fn ExitBook
  ;[1 1 1] Only exit if the book widget is open
  (Utilities|IsValid (Variables|Default|GetWidgetRef)
    (:Is%20Valid
      ;[1 1 1] Remove book widget
      (Widget|RemovefromParent (Variables|Default|GetWidgetRef))
      (Variables|Default|SetWidgetRef 0)
      ;[1 1 1] Unpause game
      (Game|SetGamePaused false))))

(fn PlayBookSFX
  (bind _sfxs (Variables|Default|GetSFXs))
  (bind _returnvalue (Audio|SpawnSoundatLocation (Utilities|Array|Get(acopy) _sfxs (Math|Random|RandomInteger (Utilities|Array|Length _sfxs))) (Transformation|GetActorLocation (Components|GetOwner)) "0, 0, 0" 1.0 1.0 0.0 0 0))
  (Class|AudioComponent|SetUISound _returnvalue true))