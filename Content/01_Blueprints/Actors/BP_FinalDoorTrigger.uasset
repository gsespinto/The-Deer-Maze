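; BP_FinalDoorTrigger is a one-shot trigger actor that opens the final door when the player walks into its box.
; On overlap with a PlayerCharacter, it spawns the PS_Mirage particle effect at its skeletal mesh, then destroys the box, audio and mesh components.
; It then sets Play on the BP_FinalDoor held in its Child Actor component, leaving the opening itself to that door.
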(event OnComponentBeginOverlap(Box)
  (params (OverlappedComponent :type Primitive%20Component%20Object%20Reference) (OtherActor :type Actor%20Object%20Reference) (OtherComp :type Primitive%20Component%20Object%20Reference) (OtherBodyIndex :type Integer) (bFromSweep :type Boolean) (SweepResult :type Hit%20Result%20Structure%20%28by%20ref%29))
  (Utilities|Casting|CastToPlayerCharacter OtherActor)
  ;[1 1 1] Spawn VFX
  (Effects|SpawnEmitteratLocation "/Game/07_VFX/PS_Mirage.PS_Mirage" (Transformation|GetWorldLocation (Variables|Default|GetSkeletalMesh)))
  ;[1 1 1] Destroy Child
  (Components|DestroyComponent (Variables|Default|GetBox))
  ;[1 1 1] Open Door
  (bind _asbp_final_door (Utilities|Casting|CastToBP_FinalDoor (Variables|/Script/Engine.ChildActorComponent|GetChildActor (Variables|Default|GetChildActor))))
  (Variables|/Game/01_Blueprints/Actors/BP_FinalDoor.BP_FinalDoor_C|SetbPlay _asbp_final_door true))

(event EventBeginPlay)

(event Collision|EventActorBeginOverlap
  (params (OtherActor :type Actor%20Object%20Reference)))

(event EventTick
  (params (DeltaSeconds :type Float%20%28single-precision%29)))

(fn ConstructionScript)