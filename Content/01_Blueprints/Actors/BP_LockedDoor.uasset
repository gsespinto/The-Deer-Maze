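; BP_LockedDoor is a door actor that swings open once when its BPInteractableDoor reports that it is open.
; Tick polls that Open flag, and a Played flag ensures the animation starts only once.
; The OpenDoor timeline then drives the relative yaw of PivotPoint to rotate the door, with no logic to close it again.
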(event EventTick
  (params (DeltaSeconds :type Float%20%28single-precision%29))
  ;[1 1 1] Garatees the door only opens once
  (if (and (Variables|/Game/01_Blueprints/Components/BP_InteractableDoor.BP_InteractableDoor_C|GetbOpen (Variables|Default|GetBP_InteractableDoor)) (not (Variables|Default|GetbPlayed)))
    (Variables|Default|SetbPlayed true)
    ;[1 1 1] Door opening code animation
    (bind _doorrotationz (Timeline|OpenDoor Play)
      (:Update
        (Transformation|SetRelativeRotation (Variables|Default|GetPivotPoint) (Math|Rotator|MakeRotator 0.0 0.0 _doorrotationz) false false)))))

(fn ConstructionScript)