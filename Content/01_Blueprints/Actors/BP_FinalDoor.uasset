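; BP_FinalDoor is a door actor, named as the final door, that swings open a single time.
; Tick polls a Play flag, which nothing in this graph sets, and uses an Opened flag so the opening fires only once.
; On opening, it plays a door sound at the actor's location and runs the OpenDoor timeline, which drives the yaw of the PivotPoint component.
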(event EventBeginPlay)

(event Collision|EventActorBeginOverlap
  (params (OtherActor :type Actor%20Object%20Reference)))

(event EventTick
  (params (DeltaSeconds :type Float%20%28single-precision%29))
  ;[1 1 1] Garantees the door only opens once
  (if (and (not (Variables|Default|GetbOpened)) (Variables|Default|GetbPlay))
    (Variables|Default|SetbOpened true)
    ;[1 1 1] SFX
    (Audio|PlaySoundatLocation "/Game/04_SFX/Doors/Open/SW_DoorOpen1.SW_DoorOpen1" (Transformation|GetActorLocation) "0, 0, 0" 1.0 1.0 0.0 0 0 0)
    ;[1 1 1] Door opening code animation
    (bind _doorrotationz (Timeline|OpenDoor Play)
      (:Update
        (Transformation|SetRelativeRotation (Variables|Default|GetPivotPoint) (Math|Rotator|MakeRotator 0.0 0.0 _doorrotationz) false false)))))

(fn ConstructionScript)