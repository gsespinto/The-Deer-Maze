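; BP_Gramophone is a gramophone actor that plays music through a jukebox interaction component.
; On BeginPlay it passes its Music audio component to BPInteractableJukebox.
; Every tick, while Music is playing, it yaws the Disk and rolls the Handle at DiskSpeed scaled by delta time.
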(event EventBeginPlay
  (Default|SetAudioComponent (Variables|Default|GetBP_InteractableJukebox) (Variables|Default|GetMusic)))

(event Collision|EventActorBeginOverlap
  (params (OtherActor :type Actor%20Object%20Reference)))

(event EventTick
  (params (DeltaSeconds :type Float%20%28single-precision%29))
  (CallFunction|RotateGramophone))

(fn ConstructionScript)

(fn RotateGramophone
  (bind _returnvalue (Utilities|Time|GetWorldDeltaSeconds))
  (bind _diskspeed (Variables|Default|GetDiskSpeed))
  (bind _returnvalue_2 (* _diskspeed _returnvalue))
  ;[1 1 1] If there's music playing
  (if (Utilities|Enum|Equal(Enum) (Audio|Components|Audio|GetPlayState (Variables|Default|GetMusic)) "Playing")
    ;[1 1 1] Rotate Disk
    (Transformation|AddRelativeRotation (Variables|Default|GetDisk) (Math|Rotator|MakeRotator 0.0 0.0 _returnvalue_2) false false)
    ;[1 1 1] Rotate Handle
    (Transformation|AddRelativeRotation (Variables|Default|GetHandle) (Math|Rotator|MakeRotator _returnvalue_2 0.0 0.0) false false)))