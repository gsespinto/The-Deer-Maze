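; Player character Blueprint that owns the HUD, toggles pausing and plays ambient orb sounds.
; BeginPlay forces VSync on and adds the HUD widget to the viewport.
; Tick updates the interact icon from the in-range interactables and counts down a randomized wait before playing a random orb sound through its audio component.
; Pause input toggles game pause, the HUD's pause display and the mouse cursor together.
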(event EventBeginPlay
  (Development|ExecuteConsoleCommand "r.VSync 1 " 0)
  (bind _returnvalue (UserInterface|CreateWidget "/Game/01_Blueprints/Widgets/WBP_HUD.WBP_HUD_C"))
  (bind _output_get (Variables|Default|SetHUD _returnvalue))
  (UserInterface|Viewport|AddtoViewport _output_get 0))

(event Collision|EventActorBeginOverlap
  (params (OtherActor :type Actor%20Object%20Reference)))

(event EventTick
  (params (DeltaSeconds :type Float%20%28single-precision%29))
  ;[1 1 1] If there are interactables within range, show interact icon, and vice versa
  (Default|InteractIconVisibility (Variables|Default|GetHUD) (> (Utilities|Array|Length (Variables|Default|GetInteractablesInRange)) 0))
  (CallFunction|PlayOrbSFX))

(event Input|ActionEvents|InputActionPause
  (params (Key :type Key%20Structure :default "None"))
  (:Pressed
    (CallFunction|TogglePause)))

(fn ConstructionScript)

(fn TogglePause
  (bind _returnvalue (Game|IsGamePaused))
  ;[1 1 1] Toggle pause state
  (Game|SetGamePaused (not _returnvalue))
  ;[1 1 1] Handle pause UI
  (Default|PauseGame (Variables|Default|GetHUD) _returnvalue)
  (Variables|/Script/Engine.PlayerController|SetbShowMouseCursor (Game|GetPlayerController 0) _returnvalue))

(fn PlayOrbSFX
  (bind _orbsfxwaitrange (Variables|Default|GetOrbSFXWaitRange))
  (bind _orbsfxs (Variables|Default|GetOrbSFXs))
  (bind _audio (Variables|Default|GetAudio))
  (if (<= (Variables|Default|GetbCurrentOrbSFXWaitTime) 0.0)
    ;[1 1 1] Play random sfx at orb's location
    (Audio|Components|Audio|SetSound _audio (Utilities|Array|Get(acopy) _orbsfxs (Math|Random|RandomInteger (Utilities|Array|Length _orbsfxs))))
    (Audio|Components|Audio|Play _audio 0.0)
    ;[1 1 1] Set random wait time from given range
    (Variables|Default|SetbCurrentOrbSFXWaitTime (Math|Random|RandomFloatinRange (.x _orbsfxwaitrange) (.y _orbsfxwaitrange)))
    (else
      ;[1 1 1] If there's wait time, tick variable
      (Variables|Default|SetbCurrentOrbSFXWaitTime (- (Variables|Default|GetbCurrentOrbSFXWaitTime) (Utilities|Time|GetWorldDeltaSeconds))))))